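; BP_Door is a proximity door that swings open while the third-person character is inside its trigger box and swings closed after they leave.
; The trigger box's overlap events set a Move flag, filtered by a cast to BP_ThirdPersonCharacter.
; Tick raises or lowers a clamped progress value at a constant rate and lerps the door's relative rotation by it, so direction can reverse mid-swing.
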(event `self.ReceiveTick`
  (params (DeltaSeconds :type "Float (single-precision)"))
  (bind _time (`self.Time`))
  (bind _returnvalue (* (`self.Delta Seconds`) 0.3))
  (bind _returnvalue_2 (+ _returnvalue _time))
  (bind _returnvalue_3 (- _time _returnvalue))
  (set `self.Delta Seconds` DeltaSeconds)
  (if (`self.Move`)
    (if (< _returnvalue_2 1.0)
      (set `self.Time` _returnvalue_2)
      (`SceneComponent.K2_SetRelativeRotation` (`self.Door`) (`KismetMathLibrary.RLerp` (struct) (struct :`Yaw` -86.0) (`self.Time`)) false false :!label _label))
    (elif (> _returnvalue_3 0.0)
      (set `self.Time` _returnvalue_3)
      (goto _label))))

(event `self.TriggerBox.OnComponentBeginOverlap`
  (params (OverlappedComponent :type "PrimitiveComponent Object Reference") (OtherActor :type "Actor Object Reference") (OtherComp :type "PrimitiveComponent Object Reference") (OtherBodyIndex :type Integer) (bFromSweep :type Boolean) (SweepResult :type "HitResult Structure (by ref)"))
  (cast `/Game/ThirdPerson/Blueprints/BP_ThirdPersonCharacter` OtherActor)
  (set `self.Move` true))

(event `self.TriggerBox.OnComponentEndOverlap`
  (params (OverlappedComponent :type "PrimitiveComponent Object Reference") (OtherActor :type "Actor Object Reference") (OtherComp :type "PrimitiveComponent Object Reference") (OtherBodyIndex :type Integer))
  (cast `/Game/ThirdPerson/Blueprints/BP_ThirdPersonCharacter` OtherActor)
  (set `self.Move` false))

(fn `UserConstructionScript`)