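; BP_BarrierDoor is a barrier that sends the third-person character back to its last checkpoint on contact, unless temporarily opened.
; Interact hides the door mesh and starts a countdown from MaxTimer, which Tick decrements and prints.
; When time expires, Tick shows the mesh again and teleports any overlapping characters.
; Overlaps beginning while the timer is inactive teleport likewise, or print a message without a valid checkpoint.
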(event `self.ReceiveTick`
  (params (DeltaSeconds :type "Float (single-precision)"))
  (bind _returnvalue (- (`self.Timer`) (`self.Delta Seconds`)))
  (set `self.Delta Seconds` DeltaSeconds)
  (if (`self.TimeActive`)
    (if (> _returnvalue 0.0)
      (bind _output_get (set `self.Timer` _returnvalue))
      (`KismetSystemLibrary.PrintString` (`KismetStringLibrary.Conv_DoubleToString` _output_get))
      (else
        (set `self.TimeActive` false)
        (set `self.Timer` 0.0)))
    (elif (not (`SceneComponent.IsVisible` (`self.SM_barrierDoor`)))
      (`SceneComponent.SetVisibility` (`self.SM_barrierDoor`) true false)
      (for _array_element (`PrimitiveComponent.GetOverlappingActors` (`self.SM_barrierDoor`) "/Game/ThirdPerson/Blueprints/BP_ThirdPersonCharacter.BP_ThirdPersonCharacter_C")
        (bind _asbp_third_person_character (cast `/Game/ThirdPerson/Blueprints/BP_ThirdPersonCharacter` _array_element))
        (bind _lastcheckpoint (`/Game/ThirdPerson/Blueprints/BP_ThirdPersonCharacter.LastCheckpoint` _asbp_third_person_character))
        (`/Engine/EditorBlueprintResources/StandardMacros.IsValid` _lastcheckpoint
          (:`Is Valid`
            (bind _trigger (`/Game/BlueRoom/Blueprints/BP_Checkpoint.Trigger` _lastcheckpoint))
            (`self.K2_TeleportTo` _asbp_third_person_character (`SceneComponent.K2_GetComponentLocation` _trigger) (`SceneComponent.K2_GetComponentRotation` _trigger)))
          (:`Is Not Valid`
            (`KismetSystemLibrary.PrintString` "No checkpoint found!")))))))

(event `/Game/BlueRoom/Blueprints/Abstract/I_Interactiv.Interact`
  (set `self.TimeActive` true)
  (set `self.Timer` (`self.MaxTimer`))
  (`SceneComponent.SetVisibility` (`self.SM_barrierDoor`) false false))

(event `self.SM_barrierDoor.OnComponentBeginOverlap`
  (params (OverlappedComponent :type "PrimitiveComponent Object Reference") (OtherActor :type "Actor Object Reference") (OtherComp :type "PrimitiveComponent Object Reference") (OtherBodyIndex :type Integer) (bFromSweep :type Boolean) (SweepResult :type "HitResult Structure (by ref)"))
  (if (not (`self.TimeActive`))
    (bind _asbp_third_person_character (cast `/Game/ThirdPerson/Blueprints/BP_ThirdPersonCharacter` OtherActor))
    (bind _lastcheckpoint (`/Game/ThirdPerson/Blueprints/BP_ThirdPersonCharacter.LastCheckpoint` _asbp_third_person_character))
    (`/Engine/EditorBlueprintResources/StandardMacros.IsValid` _lastcheckpoint
      (:`Is Valid`
        (bind _trigger (`/Game/BlueRoom/Blueprints/BP_Checkpoint.Trigger` _lastcheckpoint))
        (`self.K2_TeleportTo` _asbp_third_person_character (`SceneComponent.K2_GetComponentLocation` _trigger) (`SceneComponent.K2_GetComponentRotation` _trigger)))
      (:`Is Not Valid`
        (`KismetSystemLibrary.PrintString` "No checkpoint found!")))))

(fn `UserConstructionScript`)