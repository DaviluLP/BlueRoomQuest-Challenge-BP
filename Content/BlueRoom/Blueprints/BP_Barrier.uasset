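; BP_Barrier is a moving laser hazard that sends the third-person character back to its last checkpoint on contact.
; Tick ping-pongs a time value to lerp the laser's relative location between two marker components, DoLaser and UpLaser.
; On laser overlap, it teleports the character to the location and rotation of the saved checkpoint's trigger, or prints a message if none exists.
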(event `self.ReceiveTick`
  (params (DeltaSeconds :type "Float (single-precision)"))
  (bind _time (`self.Time`))
  (bind _returnvalue (* (`self.Delta Seconds`) 0.5))
  (bind _returnvalue_2 (+ _time _returnvalue))
  (bind _returnvalue_3 (- _time _returnvalue))
  (set `self.Delta Seconds` DeltaSeconds)
  (if (not (`self.Reverse`))
    (if (< _returnvalue_2 1.0)
      (set `self.Time` _returnvalue_2)
      (`SceneComponent.K2_SetRelativeLocation` (`self.Laser`) (`KismetMathLibrary.VLerp` (`SceneComponent.RelativeLocation` (`self.DoLaser`)) (`SceneComponent.RelativeLocation` (`self.UpLaser`)) (`self.Time`)) false false :!label _label)
      (else
        (set `self.Reverse` true)))
    (elif (> _returnvalue_3 0.0)
      (set `self.Time` _returnvalue_3)
      (goto _label)
      (else
        (set `self.Reverse` false)))))

(event `self.Laser.OnComponentBeginOverlap`
  (params (OverlappedComponent :type "PrimitiveComponent Object Reference") (OtherActor :type "Actor Object Reference") (OtherComp :type "PrimitiveComponent Object Reference") (OtherBodyIndex :type Integer) (bFromSweep :type Boolean) (SweepResult :type "HitResult Structure (by ref)"))
  (bind _asbp_third_person_character (cast `/Game/ThirdPerson/Blueprints/BP_ThirdPersonCharacter` OtherActor))
  (bind _lastcheckpoint (`/Game/ThirdPerson/Blueprints/BP_ThirdPersonCharacter.LastCheckpoint` _asbp_third_person_character))
  (`/Engine/EditorBlueprintResources/StandardMacros.IsValid` _lastcheckpoint
    (:`Is Valid`
      (bind _trigger (`/Game/BlueRoom/Blueprints/BP_Checkpoint.Trigger` _lastcheckpoint))
      (`self.K2_TeleportTo` _asbp_third_person_character (`SceneComponent.K2_GetComponentLocation` _trigger) (`SceneComponent.K2_GetComponentRotation` _trigger)))
    (:`Is Not Valid`
      (`KismetSystemLibrary.PrintString` "No Checkpoint found!"))))

(fn `UserConstructionScript`)