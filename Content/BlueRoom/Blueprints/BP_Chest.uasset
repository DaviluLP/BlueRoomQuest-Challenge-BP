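; Chest actor that opens while a BP_ThirdPersonCharacter is inside its Trigger and closes when it leaves.
; Overlap events set Activate, and Tick drives the Point component through three timed phases: a short slide, a further slide after a half-second pause, then a rotation.
; Each phase lerps on its own speed-scaled timer, which counts back down to reverse the sequence on closing.
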(event `self.ReceiveBeginPlay`
  (bind _relativelocation (`SceneComponent.RelativeLocation` (`self.Point`)))
  (set `self.StartPoint1` _relativelocation)
  (set `self.MidPoint1` (+ _relativelocation (1.5 0.0 0.0)))
  (set `self.EndPoint1` (+ _relativelocation (5.0 0.0 0.0)))
  (set `self.EndPoint2` (struct :`Pitch` 100.0)))

(event `self.ReceiveTick`
  (params (DeltaSeconds :type "Float (single-precision)"))
  (bind _returnvalue (+ (`self.Timer`) (`self.Delta Seconds`)))
  (bind _returnvalue_2 (+ (`self.Timer1`) (* (`self.Delta Seconds`) (`self.speed1`))))
  (bind _returnvalue_3 (- (`self.Timer1`) (* (`self.Delta Seconds`) (`self.speed1`))))
  (bind _returnvalue_4 (+ (`self.Timer2`) (* (`self.Delta Seconds`) (`self.speed2`))))
  (bind _returnvalue_5 (- (`self.Timer2`) (* (`self.Delta Seconds`) (`self.speed2`))))
  (bind _returnvalue_6 (+ (`self.Timer0`) (* (`self.Delta Seconds`) (`self.speed0`))))
  (bind _returnvalue_7 (- (`self.Timer0`) (* (`self.Delta Seconds`) (`self.speed0`))))
  (set `self.Delta Seconds` DeltaSeconds)
  (if (`self.Activate`)
    (if (`self.Phase0`)
      (if (< _returnvalue_6 1.0)
        (set `self.Timer0` _returnvalue_6)
        (`SceneComponent.K2_SetRelativeLocation` (`self.Point`) (`KismetMathLibrary.VLerp` (`self.StartPoint1`) (`self.MidPoint1`) (`self.Timer0`)) false false :!label _label)
        (elif (< _returnvalue 0.5)
          (set `self.Timer` _returnvalue)
          (else
            (set `self.Phase0` false))))
      (else
        ;[1 1 1] Chest Open
        (if (`self.Phase1`)
          (if (< _returnvalue_2 1.0)
            (set `self.Timer1` _returnvalue_2)
            (`SceneComponent.K2_SetRelativeLocation` (`self.Point`) (`KismetMathLibrary.VLerp` (`self.MidPoint1`) (`self.EndPoint1`) (`self.Timer1`)) false false)
            (else
              (set `self.Phase1` false)))
          (elif (< _returnvalue_4 1.0)
            (set `self.Timer2` _returnvalue_4)
            (`SceneComponent.K2_SetRelativeRotation` (`self.Point`) (`KismetMathLibrary.RLerp` (struct) (`self.EndPoint2`) (`self.Timer2`) true) false false)))))
    (elif (`self.Phase0`)
      (if (> _returnvalue_7 0.0)
        (set `self.Timer0` _returnvalue_7)
        (goto _label))
      (else
        ;[1 1 1] Chest Close
        (if (`self.Phase1`)
          (if (> _returnvalue_3 0.0)
            (set `self.Timer1` _returnvalue_3)
            (`SceneComponent.K2_SetRelativeLocation` (`self.Point`) (`KismetMathLibrary.VLerp` (`self.MidPoint1`) (`self.EndPoint1`) (`self.Timer1`)) false false)
            (else
              (set `self.Phase0` true)
              (set `self.Timer` 0.0)))
          (elif (> _returnvalue_5 0.0)
            (set `self.Timer2` _returnvalue_5)
            (`SceneComponent.K2_SetRelativeRotation` (`self.Point`) (`KismetMathLibrary.RLerp` (struct) (`self.EndPoint2`) (`self.Timer2`) true) false false)
            (else
              (set `self.Phase1` true))))))))

(event `self.Trigger.OnComponentBeginOverlap`
  (params (OverlappedComponent :type "PrimitiveComponent Object Reference") (OtherActor :type "Actor Object Reference") (OtherComp :type "PrimitiveComponent Object Reference") (OtherBodyIndex :type Integer) (bFromSweep :type Boolean) (SweepResult :type "HitResult Structure (by ref)"))
  (cast `/Game/ThirdPerson/Blueprints/BP_ThirdPersonCharacter` OtherActor)
  (set `self.Activate` true))

(event `self.Trigger.OnComponentEndOverlap`
  (params (OverlappedComponent :type "PrimitiveComponent Object Reference") (OtherActor :type "Actor Object Reference") (OtherComp :type "PrimitiveComponent Object Reference") (OtherBodyIndex :type Integer))
  (cast `/Game/ThirdPerson/Blueprints/BP_ThirdPersonCharacter` OtherActor)
  (set `self.Activate` false))

(fn `UserConstructionScript`)