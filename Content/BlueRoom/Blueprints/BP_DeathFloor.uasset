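; BP_DeathFloor is a kill floor that sends a fallen player back to a respawn point instead of destroying the character.
; When its Floor component is overlapped by a BP_ThirdPersonCharacter, it teleports that character to the trigger location and rotation of its LastCheckpoint.
; If no valid checkpoint is set, the character teleports to the first PlayerStart found in the level.
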(event `self.Floor.OnComponentBeginOverlap`
  (params (OverlappedComponent :type "PrimitiveComponent Object Reference") (OtherActor :type "Actor Object Reference") (OtherComp :type "PrimitiveComponent Object Reference") (OtherBodyIndex :type Integer) (bFromSweep :type Boolean) (SweepResult :type "HitResult Structure (by ref)"))
  (bind _asbp_third_person_character (cast `/Game/ThirdPerson/Blueprints/BP_ThirdPersonCharacter` OtherActor))
  (bind _lastcheckpoint (`/Game/ThirdPerson/Blueprints/BP_ThirdPersonCharacter.LastCheckpoint` _asbp_third_person_character))
  (`/Engine/EditorBlueprintResources/StandardMacros.IsValid` _lastcheckpoint
    (:`Is Valid`
      (bind _trigger (`/Game/BlueRoom/Blueprints/BP_Checkpoint.Trigger` _lastcheckpoint))
      (`self.K2_TeleportTo` _asbp_third_person_character (`SceneComponent.K2_GetComponentLocation` _trigger) (`SceneComponent.K2_GetComponentRotation` _trigger)))
    (:`Is Not Valid`
      (bind _returnvalue (`GameplayStatics.GetActorOfClass` "/Script/Engine.PlayerStart"))
      (`self.K2_TeleportTo` _asbp_third_person_character (`self.K2_GetActorLocation` _returnvalue) (`self.K2_GetActorRotation` _returnvalue)))))

(fn `UserConstructionScript`)