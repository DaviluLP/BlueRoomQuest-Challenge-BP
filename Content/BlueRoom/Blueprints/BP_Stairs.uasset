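; BP_Stairs is a timed staircase that moves out when Interact is called and returns when its countdown expires.
; Interact starts a countdown from StartTime, which Tick decrements and prints to screen.
; While time remains or PlayerIsOver is set, Tick lerps SMStairs toward GBStairs' relative location, otherwise back to its origin.
; TriggerBox holds the stairs out for a player character who entered during the countdown, until they leave.
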(event `self.ReceiveTick`
  (params (DeltaSeconds :type "Float (single-precision)"))
  (bind _movingtimer (`self.MovingTimer`))
  (bind _returnvalue (- (`self.Timer`) (`self.Delta Seconds`)))
  (bind _returnvalue_2 (* (`self.Delta Seconds`) 0.3))
  (bind _returnvalue_3 (+ _movingtimer _returnvalue_2))
  (bind _returnvalue_4 (- _movingtimer _returnvalue_2))
  (set `self.Delta Seconds` DeltaSeconds)
  (`|ExecutionSequence`
    (:`then_0`
      (if (or (> (`self.Timer`) 0.0) (`self.PlayerIsOver`))
        (if (< _returnvalue_3 1.0)
          (set `self.MovingTimer` _returnvalue_3)
          (`SceneComponent.K2_SetRelativeLocation` (`self.SM_Stairs`) (`KismetMathLibrary.VLerp` (0.0 0.0 0.0) (`SceneComponent.RelativeLocation` (`self.GB_Stairs`)) (`self.MovingTimer`)) false false :!label _label))
        (elif (> _returnvalue_4 0.0)
          (set `self.MovingTimer` _returnvalue_4)
          (goto _label))))
    (:`then_1`
      (if (`self.IsActiv`)
        (if (> _returnvalue 0.0)
          (bind _output_get (set `self.Timer` _returnvalue))
          (`KismetSystemLibrary.PrintString` (`KismetStringLibrary.Conv_DoubleToString` _output_get))
          (else
            (set `self.IsActiv` false)))
        (else
          (set `self.Timer` 0.0))))))

(event `/Game/BlueRoom/Blueprints/Abstract/I_Interactiv.Interact`
  (set `self.Timer` (`self.StartTime`))
  (set `self.IsActiv` true))

(event `self.TriggerBox.OnComponentBeginOverlap`
  (params (OverlappedComponent :type "PrimitiveComponent Object Reference") (OtherActor :type "Actor Object Reference") (OtherComp :type "PrimitiveComponent Object Reference") (OtherBodyIndex :type Integer) (bFromSweep :type Boolean) (SweepResult :type "HitResult Structure (by ref)"))
  (cast `/Game/ThirdPerson/Blueprints/BP_ThirdPersonCharacter` OtherActor)
  (if (`self.IsActiv`)
    (set `self.PlayerIsOver` true)))

(event `self.TriggerBox.OnComponentEndOverlap`
  (params (OverlappedComponent :type "PrimitiveComponent Object Reference") (OtherActor :type "Actor Object Reference") (OtherComp :type "PrimitiveComponent Object Reference") (OtherBodyIndex :type Integer))
  (cast `/Game/ThirdPerson/Blueprints/BP_ThirdPersonCharacter` OtherActor)
  (set `self.PlayerIsOver` false))

(fn `UserConstructionScript`)