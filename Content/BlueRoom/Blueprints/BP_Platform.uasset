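; BP_Platform is a moving platform that shuttles continuously between two marker components, Platform1 and Platform2.
; BeginPlay converts Ms, apparently metres per second, into an alpha rate using the markers' world-space distance, then prints it for debugging.
; Tick ramps Time up or down at that rate, flipping Reverse at the limits, and lerps Platform's relative location without sweep.
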(event `self.ReceiveBeginPlay`
  (bind _output_get (set `self.speed` (/ (* (`self.m/s`) 100.0) (`KismetMathLibrary.Vector_Distance` (`SceneComponent.K2_GetComponentLocation` (`self.Platform1`)) (`SceneComponent.K2_GetComponentLocation` (`self.Platform2`))))))
  (`KismetSystemLibrary.PrintString` (`KismetStringLibrary.Conv_DoubleToString` _output_get) true true (struct :`R` 0.9597 :`B` 1.0 :`A` 1.0) 5.0))

(event `self.ReceiveTick`
  (params (DeltaSeconds :type "Float (single-precision)"))
  (bind _time (`self.Time`))
  (bind _returnvalue (* (`self.Delta Seconds`) (`self.speed`)))
  (set `self.Delta Seconds` DeltaSeconds)
  (if (`self.Reverse`)
    (if (< _time 1.0)
      (set `self.Time` (+ _time _returnvalue))
      (`SceneComponent.K2_SetRelativeLocation` (`self.Platform`) (`KismetMathLibrary.VLerp` (`SceneComponent.RelativeLocation` (`self.Platform1`)) (`SceneComponent.RelativeLocation` (`self.Platform2`)) (`self.Time`)) false false :!label _label)
      (else
        (set `self.Reverse` false)))
    (elif (> _time 0.0)
      (set `self.Time` (- _time _returnvalue))
      (goto _label)
      (else
        (set `self.Reverse` true)))))

(fn `UserConstructionScript`)